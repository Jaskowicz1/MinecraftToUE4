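; Game mode that builds a block structure in the level from the lines of Pyramid.txt, apparently data brought over from Minecraft.
; ShowBlocks splits each comma-separated line into type and coordinates, scales them by 100 and spawns a Block_BP.
; The Things collection records processed lines to skip duplicates.
; With DevelopementMode on, Tick re-reads the file through a one-second Delay, adding new lines live but never removing blocks.
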(event `self.ReceiveBeginPlay`
  (`self.Show Blocks`))

(event `self.ReceiveTick`
  (params (DeltaSeconds :type "Float (single-precision)"))
  (if (`self.DevelopementMode`)
    (`KismetSystemLibrary.Delay` 1.0)
    (`self.Show Blocks`)))

(event `Show Blocks`
  (bind _returnvalue (`self.getLines` "Pyramid.txt"))
  (for _array_element _returnvalue
    (if (not (`KismetArrayLibrary.Array_Contains` (`self.Things`) _array_element))
      (`KismetArrayLibrary.Array_Add` (`self.Things`) _array_element)
      (bind (_lefts _rights) (`KismetStringLibrary.Split` _array_element ","))
      (bind (_lefts_2 _rights_2) (`KismetStringLibrary.Split` _rights ","))
      (bind (_lefts_3 _rights_3) (`KismetStringLibrary.Split` _rights_2 ","))
      (`|SpawnActorFromClass` "/Game/Blueprints/Block_BP.Block_BP_C" (`KismetMathLibrary.MakeTransform` (`KismetMathLibrary.MakeVector` (* (`KismetStringLibrary.Conv_StringToDouble` _lefts_2) 100.0) (* (`KismetStringLibrary.Conv_StringToDouble` _lefts_3) 100.0) (* (`KismetStringLibrary.Conv_StringToDouble` _rights_3) 100.0))) "Undefined" "OverrideRootScale" null _lefts null))))

(fn `UserConstructionScript`)